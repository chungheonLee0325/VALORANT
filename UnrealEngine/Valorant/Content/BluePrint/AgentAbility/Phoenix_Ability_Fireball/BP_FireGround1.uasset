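; BP_FireGround1 is the ground fire actor of Phoenix's Fireball ability, adding spawn and decay audio to its parent class.
; BeginPlay calls the parent, then MulticastSpawnSFX plays the molotov ground-spawn sound at the actor's location.
; Destroyed calls the parent, then MulticastDestroySFX plays the zone-decay sound at the same spot.
; The graph holds only this audio logic, and the construction script is empty.
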(event `self.ReceiveBeginPlay`
  (`parent.ReceiveBeginPlay`)
  (`self.MulticastSpawnSFX`))

(event `MulticastSpawnSFX`
  (`GameplayStatics.PlaySoundAtLocation` "/Game/Resource/Agent/Phoenix/Ability/SFX/_Char_Phoenix/Abil_C/Phoenix_Q_GroundSpawn_Molotov_Explo_Comp_TP_Alt2_1__SFX__Cue.Phoenix_Q_GroundSpawn_Molotov_Explo_Comp_TP_Alt2_1__SFX__Cue" (`self.K2_GetActorLocation`) (struct) 1.0 1.0 0.0 null null null null))

(event `self.ReceiveDestroyed`
  (`parent.ReceiveDestroyed`)
  (`self.MulticastDestroySFX`))

(event `MulticastDestroySFX`
  (`GameplayStatics.PlaySoundAtLocation` "/Game/Resource/Agent/Phoenix/Ability/SFX/_Char_Phoenix/Abil_C/Phoenix_Molotov_ZoneDecay_TP_02__SFX__Cue.Phoenix_Molotov_ZoneDecay_TP_02__SFX__Cue" (`self.K2_GetActorLocation`) (struct) 1.0 1.0 0.0 null null null null))

(fn `UserConstructionScript`)