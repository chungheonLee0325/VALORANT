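; Character that fires agent-ability projectiles from number keys, each key spawning a different type such as fireball, cloudball, flashbang, knife, grenade or incendiary bomb.
; Each press deprojects the screen center of player 0 to get the spawn location and aim direction, then spawns the projectile with itself as Instigator, ignoring collision.
; Two keys share the flashbang class and differ only in the boolean passed to its ActiveProjectileMovement call.
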(event `Key|One`
  (params (Key :type "Key Structure"))
  (bind _returnvalue (`GameplayStatics.GetPlayerController` 0))
  (bind (_sizex _sizey) (`PlayerController.GetViewportSize` _returnvalue))
  (bind (_worldposition _worlddirection) (`GameplayStatics.DeprojectScreenToWorld` _returnvalue (`KismetMathLibrary.MakeVector2D` (* _sizex 0.5) (* _sizey 0.5))))
  (:`Pressed`
    (`|SpawnActorFromClass` "/Game/BluePrint/AgentAbility/Phoenix_Ability_Fireball/BP_Fireball.BP_Fireball_C" (`KismetMathLibrary.MakeTransform` _worldposition (`KismetMathLibrary.MakeRotFromX` _worlddirection)) "AlwaysSpawn" "MultiplyWithRoot" null self)))

(event `Key|Two`
  (params (Key :type "Key Structure"))
  (bind _returnvalue (`GameplayStatics.GetPlayerController` 0))
  (bind (_sizex _sizey) (`PlayerController.GetViewportSize` _returnvalue))
  (bind (_worldposition _worlddirection) (`GameplayStatics.DeprojectScreenToWorld` _returnvalue (`KismetMathLibrary.MakeVector2D` (* _sizex 0.5) (* _sizey 0.5))))
  (:`Pressed`
    (`|SpawnActorFromClass` "/Game/BluePrint/AgentAbility/Jett_Ability_Windball/BP_Cloudball.BP_Cloudball_C" (`KismetMathLibrary.MakeTransform` _worldposition (`KismetMathLibrary.MakeRotFromX` _worlddirection)) "AlwaysSpawn" "MultiplyWithRoot" null self)))

(event `Key|Three`
  (params (Key :type "Key Structure"))
  (bind _returnvalue (`GameplayStatics.GetPlayerController` 0))
  (bind (_sizex _sizey) (`PlayerController.GetViewportSize` _returnvalue))
  (bind (_worldposition _worlddirection) (`GameplayStatics.DeprojectScreenToWorld` _returnvalue (`KismetMathLibrary.MakeVector2D` (* _sizex 0.5) (* _sizey 0.5))))
  (:`Pressed`
    (bind _returnvalue_2 (`|SpawnActorFromClass` "/Game/BluePrint/AgentAbility/KayO_Ability_Flashbang/BP_Flashbang.BP_Flashbang_C" (`KismetMathLibrary.MakeTransform` _worldposition (`KismetMathLibrary.MakeRotFromX` _worlddirection)) "AlwaysSpawn" "MultiplyWithRoot" null self))
    (`Flashbang.ActiveProjectileMovement` _returnvalue_2 false)))

(event `Key|Four`
  (params (Key :type "Key Structure"))
  (bind _returnvalue (`GameplayStatics.GetPlayerController` 0))
  (bind (_sizex _sizey) (`PlayerController.GetViewportSize` _returnvalue))
  (bind (_worldposition _worlddirection) (`GameplayStatics.DeprojectScreenToWorld` _returnvalue (`KismetMathLibrary.MakeVector2D` (* _sizex 0.5) (* _sizey 0.5))))
  (:`Pressed`
    (bind _returnvalue_2 (`|SpawnActorFromClass` "/Game/BluePrint/AgentAbility/KayO_Ability_Flashbang/BP_Flashbang.BP_Flashbang_C" (`KismetMathLibrary.MakeTransform` _worldposition (`KismetMathLibrary.MakeRotFromX` _worlddirection)) "AlwaysSpawn" "MultiplyWithRoot" null self))
    (`Flashbang.ActiveProjectileMovement` _returnvalue_2 true)))

(event `Key|Five`
  (params (Key :type "Key Structure"))
  (bind _returnvalue (`GameplayStatics.GetPlayerController` 0))
  (bind (_sizex _sizey) (`PlayerController.GetViewportSize` _returnvalue))
  (bind (_worldposition _worlddirection) (`GameplayStatics.DeprojectScreenToWorld` _returnvalue (`KismetMathLibrary.MakeVector2D` (* _sizex 0.5) (* _sizey 0.5))))
  (:`Pressed`
    (`|SpawnActorFromClass` "/Game/BluePrint/AgentAbility/KayO_Ability_Knife/BP_KayoKnife.BP_KayoKnife_C" (`KismetMathLibrary.MakeTransform` _worldposition (`KismetMathLibrary.MakeRotFromX` _worlddirection)) "AlwaysSpawn" "MultiplyWithRoot" null self)))

(event `Key|Six`
  (params (Key :type "Key Structure"))
  (bind _returnvalue (`GameplayStatics.GetPlayerController` 0))
  (bind (_sizex _sizey) (`PlayerController.GetViewportSize` _returnvalue))
  (bind (_worldposition _worlddirection) (`GameplayStatics.DeprojectScreenToWorld` _returnvalue (`KismetMathLibrary.MakeVector2D` (* _sizex 0.5) (* _sizey 0.5))))
  (:`Pressed`
    (`|SpawnActorFromClass` "/Game/BluePrint/AgentAbility/KayO_Ability_Grenade/BP_KayoGrenade.BP_KayoGrenade_C" (`KismetMathLibrary.MakeTransform` _worldposition (`KismetMathLibrary.MakeRotFromX` _worlddirection)) "AlwaysSpawn" "MultiplyWithRoot" null self)))

(event `Key|Seven`
  (params (Key :type "Key Structure"))
  (bind _returnvalue (`GameplayStatics.GetPlayerController` 0))
  (bind (_sizex _sizey) (`PlayerController.GetViewportSize` _returnvalue))
  (bind (_worldposition _worlddirection) (`GameplayStatics.DeprojectScreenToWorld` _returnvalue (`KismetMathLibrary.MakeVector2D` (* _sizex 0.5) (* _sizey 0.5))))
  (:`Pressed`
    (`|SpawnActorFromClass` "/Game/BluePrint/AgentAbility/Brimstone_Ability_Incendiary/BP_IncendiaryBomb.BP_IncendiaryBomb_C" (`KismetMathLibrary.MakeTransform` _worldposition (`KismetMathLibrary.MakeRotFromX` _worlddirection)) "AlwaysSpawn" "MultiplyWithRoot" null self)))

(fn `UserConstructionScript`
  (`parent.UserConstructionScript`))