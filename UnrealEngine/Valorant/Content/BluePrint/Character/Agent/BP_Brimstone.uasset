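; Brimstone agent character Blueprint that adds the agent input mapping context for the local player and plays a kill sound locally.
; Holding I records microphone audio, saves it as a WAV and sends it, while toggling recording on the match map HUD.
; Number keys act as test shortcuts for ability purchase, credits, and server-applied fast and dead gameplay effects.
; Skill input events are empty, with leftover debug nodes disconnected.
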(event `self.ReceiveBeginPlay`)

(event `self.ReceiveControllerChanged`
  (params (OldController :type "Controller Object Reference") (NewController :type "Controller Object Reference"))
  ; Default
  (if (`self.IsLocallyControlled`)
    (bind `_as플레이어_컨트롤러` (cast `PlayerController` NewController))
    (`EnhancedInputSubsystemInterface.AddMappingContext` (pcsubsystem `EnhancedInputLocalPlayerSubsystem` `_as플레이어_컨트롤러`) "/Game/BluePrint/Character/Input/IMC_AgentDefault.IMC_AgentDefault" 0 (struct))))

(event `EnhancedInput|/Game/BluePrint/Character/Input/Actions/Ability/IA_Q`
  (params (ActionValue :type Boolean) (ElapsedSeconds :type "Float (double-precision)") (TriggeredSeconds :type "Float (double-precision)") (InputAction :type "InputAction Object Reference" :default "/Game/BluePrint/Character/Input/Actions/Ability/IA_Q.IA_Q"))
  ; Skill Input
)

(event `EnhancedInput|/Game/BluePrint/Character/Input/Actions/Ability/IA_E`
  (params (ActionValue :type Boolean) (ElapsedSeconds :type "Float (double-precision)") (TriggeredSeconds :type "Float (double-precision)") (InputAction :type "InputAction Object Reference" :default "/Game/BluePrint/Character/Input/Actions/Ability/IA_E.IA_E"))
  ; Skill Input
)

(event `EnhancedInput|/Game/BluePrint/Character/Input/Actions/Default/IA_LeftClickStart`
  (params (ActionValue :type Boolean) (ElapsedSeconds :type "Float (double-precision)") (TriggeredSeconds :type "Float (double-precision)") (InputAction :type "InputAction Object Reference" :default "/Game/BluePrint/Character/Input/Actions/Default/IA_LeftClickStart.IA_LeftClickStart"))
  ; Default
)

(event `EnhancedInput|/Game/BluePrint/Character/Input/Actions/Ability/IA_C`
  (params (ActionValue :type Boolean) (ElapsedSeconds :type "Float (double-precision)") (TriggeredSeconds :type "Float (double-precision)") (InputAction :type "InputAction Object Reference" :default "/Game/BluePrint/Character/Input/Actions/Ability/IA_C.IA_C"))
  ; Skill Input
)

(event `EnhancedInput|/Game/BluePrint/Character/Input/Actions/Default/IA_RIghtClick`
  (params (ActionValue :type Boolean) (ElapsedSeconds :type "Float (double-precision)") (TriggeredSeconds :type "Float (double-precision)") (InputAction :type "InputAction Object Reference" :default "/Game/BluePrint/Character/Input/Actions/Default/IA_RIghtClick.IA_RIghtClick"))
  ; Default
)

(event `EnhancedInput|/Game/BluePrint/Character/Input/Actions/Ability/IA_X`
  (params (ActionValue :type Boolean) (ElapsedSeconds :type "Float (double-precision)") (TriggeredSeconds :type "Float (double-precision)") (InputAction :type "InputAction Object Reference" :default "/Game/BluePrint/Character/Input/Actions/Ability/IA_X.IA_X"))
  ; Skill Input
)

(event `Key|Zero`
  (params (Key :type "Key Structure"))
  (:`Pressed`
    (bind _asagent_player_controller (cast `AgentPlayerController` (`GameplayStatics.GetPlayerController` 0)))
    (`AgentPlayerController.RequestPurchaseAbility` _asagent_player_controller 1)))

(event `Key|I`
  (params (Key :type "Key Structure"))
  (bind _returnvalue (`MatchPlayerController.GetMatchMapHud` (`self.GetPC`)))
  ; ai
  (:`Pressed`
    (`SynthComponent.Start` (`self.AudioCapture`))
    (`AudioMixerBlueprintLibrary.StartRecordingOutput` 0.0 null)
    (bind _asmatch_map_hud (cast `MatchMapHUD` _returnvalue))
    (`MatchMapHUD.StartRecording` _asmatch_map_hud))
  (:`Released`
    (`SynthComponent.Stop` (`self.AudioCapture`))
    (`AudioMixerBlueprintLibrary.StopRecordingOutput` "WavFile" "UserVoiceInput" "../UserVoiceInput/" null null)
    (`self.SendWavFileDirectly`)
    (bind _asmatch_map_hud_2 (cast `MatchMapHUD` _returnvalue))
    (`MatchMapHUD.EndRecording` _asmatch_map_hud_2)))

(event `Key|Nine`
  (params (Key :type "Key Structure"))
  (:`Pressed`
    (bind _asagent_player_state (cast `AgentPlayerState` (`self.PlayerState`)))
    (`CreditComponent.AddCredits` (`AgentPlayerState.GetCreditComponent` _asagent_player_state) 1000)))

(event `Key|Five`
  (params (Key :type "Key Structure"))
  (:`Pressed`
    (if (`self.IsLocallyControlled`)
      (`self.ServerApplyGE` "/Game/BluePrint/GAS/Effects/GE_Fast.GE_Fast_C"))))

(event `Key|Six`
  (params (Key :type "Key Structure"))
  (:`Pressed`
    (if (`self.IsLocallyControlled`)
      (`self.ServerApplyGE` "/Game/BluePrint/GAS/Effects/GE_Dead.GE_Dead_C"))))

(event `self.OnKill`
  (if (`self.IsLocallyControlled`)
    (`GameplayStatics.PlaySound2D` "/Game/Resource/Audio/Kill/kill_1.kill_1" 1.0 1.0 0.0 null null)))

(fn `UserConstructionScript`)