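; Phoenix's C-ability Blaze spline wall actor, adding spawn and decay audio on top of its parent class.
; BeginPlay calls the parent, then MulticastSpawnSFX plays the looping wall cue at the actor's location.
; Destroyed calls the parent, then MulticastDestroySFX plays the decay cue there.
; The loop is fire-and-forget with no stored audio component, so this Blueprint never stops it explicitly.
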(event `self.ReceiveBeginPlay`
  (`parent.ReceiveBeginPlay`)
  (`self.MulticastSpawnSFX`))

(event `MulticastSpawnSFX`
  (`GameplayStatics.PlaySoundAtLocation` "/Game/Resource/Agent/Phoenix/Ability/SFX/_Char_Phoenix/Abil_Q/Phoenix_Wall_Loop_TP__SFX__Cue.Phoenix_Wall_Loop_TP__SFX__Cue" (`self.K2_GetActorLocation`) (struct) 1.0 1.0 0.0 null null null null))

(event `self.ReceiveDestroyed`
  (`parent.ReceiveDestroyed`)
  (`self.MulticastDestroySFX`))

(event `MulticastDestroySFX`
  (`GameplayStatics.PlaySoundAtLocation` "/Game/Resource/Agent/Phoenix/Ability/SFX/_Char_Phoenix/Abil_Q/Phoenix__Wall_Decay_TP_v2_2__SFX__Cue.Phoenix__Wall_Decay_TP_v2_2__SFX__Cue" (`self.K2_GetActorLocation`) (struct) 1.0 1.0 0.0 null null null null))

(fn `UserConstructionScript`)